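; Neko_BP is the 2D player cat character for Neko Run, choosing its flipbook animation from movement and death state.
; Every Tick, UpdateAnimation selects run, slide (crouching), jump or fall from ground state and vertical velocity, then sets it on the Sprite via UpdateFlipBook.
; While IsPlayerDead is set, it shows the dead flipbook and calls GameEnds on MyNekoRunGameModeBase_BP, repeating every frame.
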(event Custom|UpdateAnimation
  (if (Variables|Default|GetIsPlayerDead)
    (CallFunction|UpdateFlipBook "/Game/Assets/Flipbooks/Flipbook_Dead.Flipbook_Dead")
    (bind _asmy_neko_run_game_mode_base_bp (Utilities|Casting|CastToMyNekoRunGameModeBase_BP (Game|GetGameMode)))
    (Default|GameEnds _asmy_neko_run_game_mode_base_bp)
    (elif (AI|Components|NavMovement|IsMovingonGround (Variables|Character|GetCharacterMovement))
      (if (AI|Components|NavMovement|IsCrouching (Variables|Character|GetCharacterMovement))
        (CallFunction|UpdateFlipBook "/Game/Assets/Flipbooks/Flipbook_Slide.Flipbook_Slide")
        (else
          (CallFunction|UpdateFlipBook "/Game/Assets/Flipbooks/Flipbook_Run.Flipbook_Run")))
      (elif (> (.z (Transformation|GetVelocity)) 0.0)
        (CallFunction|UpdateFlipBook "/Game/Assets/Flipbooks/Flipbook_Jump.Flipbook_Jump")
        (else
          (CallFunction|UpdateFlipBook "/Game/Assets/Flipbooks/Flipbook_Fall.Flipbook_Fall"))))))

(event EventBeginPlay)

(event Collision|EventActorBeginOverlap
  (params (OtherActor :type Actor%20Object%20Reference)))

(event EventTick
  (params (DeltaSeconds :type Float%20%28single-precision%29))
  (CallFunction|UpdateAnimation))

(fn ConstructionScript)

(fn UpdateFlipBook
  (params (FlipBookAnimation :type Paper%20Flipbook%20Object%20Reference))
  (Sprite|SetFlipbook (Variables|Default|GetSprite) FlipBookAnimation))