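; Game mode for NekoRun that tracks the run's distance and handles the game-over state.
; BeginPlay creates the BP_Game_HUD widget and adds it to the viewport.
; Until game over, Tick adds delta time plus a constant to the total distance, so it grows with frame rate, and sends a scaled value to the HUD.
; GameEnds stops the count, shows the restart button and reveals the mouse cursor.
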(event Custom|GameEnds
  (Variables|Default|SetGameOver true)
  (Default|ShowRestartButton (Variables|Default|GetGameHud))
  (Variables|/Script/Engine.PlayerController|SetbShowMouseCursor (Game|GetPlayerController 0) true))

(event EventBeginPlay
  (Variables|Default|SetGameOver false)
  (bind _returnvalue (UserInterface|CreateWidget "/Game/BluePrints/BP_Game_HUD.BP_Game_HUD_C" (Game|GetPlayerController 0)))
  (bind _output_get (Variables|Default|SetGameHud _returnvalue))
  (UserInterface|Viewport|AddtoViewport _output_get 0))

(event EventTick
  (params (DeltaSeconds :type Float%20%28single-precision%29))
  (if (not (Variables|Default|GetGameOver))
    (bind _output_get (Variables|Default|SetTotalDistance (+ (Variables|Default|GetTotalDistance) (+ DeltaSeconds 1e+03))))
    (Default|UpdateDistance (Variables|Default|GetGameHud) (/ _output_get 1e+02))))

(fn ConstructionScript)